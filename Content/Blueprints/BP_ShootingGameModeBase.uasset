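; Game mode Blueprint for a shooting game that tracks the current score and a persistent high score.
; AddScore increments Score and, when it beats HighScore, calls GameSave, which writes a new BP_SaveGame object to a slot.
; GameLoad returns the saved high score, or 0 if no save exists.
; BeginPlay is empty; the score widget, high-score loading and game-only input setup are disconnected and never run.
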(event EventBeginPlay)

(event EventTick
  (params (DeltaSeconds :type Float%20%28single-precision%29)))

(fn ConstructionScript)

(fn AddScore
  ;[1 1 1] 점수를 1점 증가시키고싶다.
  (bind _output_get (Variables|Default|SetScore (+ (Variables|Default|GetScore) 1)))
  ;[1 1 1] 만약 Score가 HighScore보다 크다면 HighScore = Score 하고싶다.
  (if (> _output_get (Variables|Default|GetHighScore))
    (bind _output_get_2 (Variables|Default|SetHighScore _output_get))
    (CallFunction|GameSave _output_get_2)))

(fn GameSave
  (params (In_HighSocre :type Integer))
  (Utilities|FlowControl|Sequence
    (:then_0
      ;[1 1 1] SaveGame 인스턴스 생성
      (bind _returnvalue (SaveGame|CreateSaveGameObject "/Game/Blueprints/BP_SaveGame.BP_SaveGame_C"))
      (Variables|Default|SetSaveGameInstance _returnvalue))
    (:then_1
      ;[1 1 1] 생성한 인스턴스에 저장할 값을 복사
      (Variables|/Game/Blueprints/BP_SaveGame.BP_SaveGame_C|SetHighScore_Save (Variables|Default|GetSaveGameInstance) In_HighSocre))
    (:then_2
      ;[1 1 1] 파일에 저장
      (SaveGame|SaveGametoSlot (Variables|Default|GetSaveGameInstance) (Variables|Default|GetSlotName)))))

(fn GameLoad
  ;[1 1 1] GameSlot을 Load하고 그안에 들어있는 값을 반환하고싶다.
  (Utilities|FlowControl|Sequence
    (:then_0
      (bind _returnvalue (SaveGame|DoesSaveGameExist (Variables|Default|GetSlotName)))
      (if (not _returnvalue)
        (return 0)))
    (:then_1
      (bind _returnvalue_2 (SaveGame|LoadGamefromSlot (Variables|Default|GetSlotName)))
      (bind _asbp_save_game (Utilities|Casting|CastToBP_SaveGame _returnvalue_2))
      (return (Variables|/Game/Blueprints/BP_SaveGame.BP_SaveGame_C|GetHighScore_Save _asbp_save_game)))))