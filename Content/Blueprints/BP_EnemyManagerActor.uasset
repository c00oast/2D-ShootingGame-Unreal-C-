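; BP_EnemyManagerActor is an enemy spawner whose MakeEnemy function spawns BP_EnemyActor at its arrow component's transform, ignoring collisions.
; The graph keeps four alternative periodic triggers based on CreateTime0: Delay, timer by function name, timer by event, and a Tick accumulator that checks for a valid player pawn.
; All four are disconnected, with BeginPlay and Tick empty, so the blueprint does not start spawning by itself.
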(event Custom|Event%20MakeEnemy
  ;[1 1 1] 이벤트를 타이머에 등록하기
  (CallFunction|MakeEnemy))

(event EventBeginPlay
  ;[1 1 1] 함수를 타이머에 등록하기
)

(event Collision|EventActorBeginOverlap
  (params (OtherActor :type Actor%20Object%20Reference)))

(event EventTick
  (params (DeltaSeconds :type Float%20%28single-precision%29))
  ;[1 1 1] 1. 시간이 흐르다가
  ; 2. 만약 현재시간이 생성시간을 초과하면
  ; 3. 적공장에서 적을 생성해서 화살표 위치에 배치하고싶다.
  ; 4. 현재시간을 0으로 초기화 하고싶다.
)

(fn ConstructionScript)

(fn MakeEnemy
  (bind _arrowcomp (Variables|Default|GetarrowComp))
  (bind _returnvalue (Transformation|GetWorldTransform _arrowcomp))
  (Game|SpawnActorfromClass "/Game/Blueprints/BP_EnemyActor.BP_EnemyActor_C" (Math|Transform|MakeTransform (.location _returnvalue) (.rotation _returnvalue) "1,1,1") "AlwaysSpawn" 0 0))