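; BP_BulletActor is a bullet actor for a shooting game, but its BeginPlay, overlap and Tick events are all empty.
; Disconnected movement nodes would advance it along its forward vector by speed times delta time, without sweep.
; Disconnected hit nodes would spawn an explosion at an overlapped BP_EnemyActor, destroy it, add score through BP_ShootingGameModeBase, then destroy the bullet.
; As wired, none of this Blueprint logic runs.
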(event EventBeginPlay)

(event Collision|EventActorBeginOverlap
  (params (OtherActor :type Actor%20Object%20Reference))
  ;[1 1 1] Bullet이 Enemy와 부딪혔다!!! VFX만들고 너죽고 나죽자
)

(event EventTick
  (params (DeltaSeconds :type Float%20%28single-precision%29))
  ;[1 1 1] P = P0 + v(방향 * speed) * t
)

(fn ConstructionScript)